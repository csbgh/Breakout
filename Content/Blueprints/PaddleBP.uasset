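; Paddle actor with a cartoon face that reacts to the nearest Ball.
; Each tick it searches all Ball actors for the closest and passes it to the eye and mouth functions.
; Both eyes shift slightly from their PaddleSprite sockets along the direction to that ball, in actor-local coordinates.
; The mouth sprite turns happy when the ball is within a short distance and sad otherwise.
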(event EventBeginPlay)

(event Collision|EventActorBeginOverlap
  (params (OtherActor :type Actor%20Object%20Reference)))

(event EventTick
  (params (DeltaSeconds :type Float%20%28single-precision%29))
  (bind _closest (CallFunction|GetClosestBall))
  (CallFunction|SetEyeLocation "EyeLeft" (Variables|Default|GetEyeLeft) _closest)
  (CallFunction|SetEyeLocation "EyeRight" (Variables|Default|GetEyeRight) _closest)
  (CallFunction|SetMouthSprite _closest))

(fn ConstructionScript)

(fn GetClosestBall
  (bind _outactors (Actor|GetAllActorsOfClass "/Script/Breakout.Ball"))
  (for _array_element _outactors
    (if (< (Transformation|GetDistanceTo _array_element self) (LocalVariables|GetClosestDistance))
      (LocalVariables|SetClosestDistance (Transformation|GetDistanceTo _array_element self))
      (LocalVariables|SetClosestBall _array_element)))
  (return (LocalVariables|GetClosestBall)))

(fn SetEyeLocation
  (params (EyeSocketName :type Name) (EyeComponent :type Scene%20Component%20Object%20Reference) (Ball :type Ball%20Object%20Reference))
  (Transformation|SetRelativeLocation EyeComponent (+ (Math|Transform|InverseTransformLocation (Transformation|GetActorTransform self) (Transformation|GetSocketLocation (Variables|Default|GetPaddleSprite) EyeSocketName)) (Math|Vector|ClampVectorSize (* (Math|Vector|GetUnitDirection(Vector) (Transformation|GetActorLocation self) (Transformation|GetActorLocation Ball)) 2.0) -1.0 1.0)) false false))

(fn SetMouthSprite
  (params (Ball :type Ball%20Object%20Reference))
  (if (< (Transformation|GetDistanceTo Ball self) 75.0)
    (Rendering|Components|Sprite|SetSprite (Variables|Default|GetMouth) "/Game/Sprites/PaddleMouthHappy.PaddleMouthHappy")
    (else
      (Rendering|Components|Sprite|SetSprite (Variables|Default|GetMouth) "/Game/Sprites/PaddleMouthSad.PaddleMouthSad"))))